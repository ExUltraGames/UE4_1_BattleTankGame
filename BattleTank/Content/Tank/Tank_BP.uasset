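; Tank pawn Blueprint that sets up a tank's components, health bar and camera switching.
; BeginPlay hands barrel and turret to TankAiming, both tracks to TankMovement, and a self reference to the HealthBar_UI widget.
; Two input actions toggle first-person or barrel cameras against the third-person camera.
; Axis and track-hit events are empty, with leftover disconnected logic; a comment notes ballistic input moved to Tank.cpp.
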(event EventBeginPlay
  (Class|TankAimingComponent|Initialise (Variables|Default|GetTankAiming_) (Variables|Default|GetTankBarrel_) (Variables|Default|GetTankTurret))
  (Class|TankMovementComponent|Initialise (Variables|Default|GetTankMovement) (Variables|Default|GetTankTrackL) (Variables|Default|GetTankTrackR))
  (CallFunction|InitialiseHealthBarWidget))

(event Collision|EventActorBeginOverlap
  (params (OtherActor :type Actor%20Object%20Reference)))

(event EventTick
  (params (DeltaSeconds :type Float%20%28single-precision%29))
  ;[1 1 1] Check Health status is working
)

(event OnComponentHit(TankTrackRight)
  (params (HitComponent :type Primitive%20Component%20Object%20Reference) (OtherActor :type Actor%20Object%20Reference) (OtherComp :type Primitive%20Component%20Object%20Reference) (NormalImpulse :type Vector :default "0, 0, 0") (Hit :type Hit%20Result%20Structure%20%28by%20ref%29))
  ;[1 1 1] OnComponentHIt Log
)

(event Input|ActionEvents|InputActionCameraView
  (params (Key :type Key%20Structure :default "None"))
  ;[1 1 1] Camera Swopping
  (:Pressed
    (Components|Activation|ToggleActive (Variables|Default|GetCamera1stPerson))
    (Components|Activation|ToggleActive (Variables|Default|GetCamera3rdPerson))))

(event Input|ActionEvents|InputActionFire
  (params (Key :type Key%20Structure :default "None"))
  ;[1 1 1] Ballistic Binding: moved to Tank.cpp
)

(event Input|ActionEvents|InputActionCameraBarrelView
  (params (Key :type Key%20Structure :default "None"))
  (:Pressed
    (Components|Activation|ToggleActive (Variables|Default|GetCameraBarrel))
    (Components|Activation|ToggleActive (Variables|Default|GetCamera3rdPerson))))

(event Input|AxisEvents|InputAxisAimAzimuth
  (params (AxisValue :type Float%20%28single-precision%29))
  ;[1 1 1] Ballistic Binding: moved to Tank.cpp
)

(event Input|AxisEvents|InputAxisAimAltitude
  (params (AxisValue :type Float%20%28single-precision%29))
  ;[1 1 1] Ballistic Binding: moved to Tank.cpp
)

(event Input|AxisEvents|InputAxisLeftTrackThrottle
  (params (AxisValue :type Float%20%28single-precision%29))
  ;[1 1 1] MOvement Input Binding
)

(event Input|AxisEvents|InputAxisRightTrackThrottle
  (params (AxisValue :type Float%20%28single-precision%29))
  ;[1 1 1] MOvement Input Binding
)

(event Input|AxisEvents|InputAxisMoveForward
  (params (AxisValue :type Float%20%28single-precision%29))
  ;[1 1 1] MOvement Input Binding
)

(event Input|AxisEvents|InputAxisTurnRight
  (params (AxisValue :type Float%20%28single-precision%29))
  ;[1 1 1] MOvement Input Binding
)

(fn ConstructionScript)

(fn InitialiseHealthBarWidget
  (bind _ashealth_bar_ui (Utilities|Casting|CastToHealthBar_UI (UserInterface|GetUserWidgetObject (Variables|Default|GetHealthWidget))))
  (Variables|/Game/UI/HealthBar_UI.HealthBar_UI_C|SetTank%20Ref _ashealth_bar_ui self)
  (return))